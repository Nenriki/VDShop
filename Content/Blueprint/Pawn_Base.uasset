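; Base pawn that shows the UI_Base widget on BeginPlay and hides a keyboard easter egg that displays UI_UWU.
; Pressing Enter five or more times arms a chain of Gates that unlocks through the key order B, E, B, O, U.
; Each Gate's exit opens the next, while the letter keys close other Gates to break out-of-order input.
; A RemoveUI event removes a given widget from its parent.
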(event `self.ReceiveBeginPlay`
  ;[0.3837 0.3884 1] Add Widget to viewport
  (bind _returnvalue (`|CreateWidget` "/Game/Blueprint/UI_Base.UI_Base_C"))
  (`UserWidget.AddToViewport` _returnvalue 0))

(event `Key|B`
  (params (Key :type "Key Structure"))
  ;[1 1 1 0.568] Easter Egg
  (:`Pressed`
    (`|ExecutionSequence`
      (:`then_0`
        (goto _label_5 :!via `Close`))
      (:`then_1`
        (`/Engine/EditorBlueprintResources/StandardMacros.Gate` true :!label _label
          (:`Exit`
            (goto _label_4 :!via `Open`))))
      (:`then_2`
        (`/Engine/EditorBlueprintResources/StandardMacros.Gate` true :!label _label_2
          (:`Exit`
            (goto _label_3 :!via `Open`)))))))

(event `Key|E`
  (params (Key :type "Key Structure"))
  ;[1 1 1 0.568] Easter Egg
  (:`Pressed`
    (`|ExecutionSequence`
      (:`then_0`
        (goto _label_4 :!via `Close`))
      (:`then_1`
        (goto _label_2 :!via `Close`))
      (:`then_2`
        (goto _label_5 :!via `Close`))
      (:`then_3`
        (`/Engine/EditorBlueprintResources/StandardMacros.Gate` true :!label _label_3
          (:`Exit`
            (goto _label :!via `Open`)))))))

(event `Key|O`
  (params (Key :type "Key Structure"))
  ;[1 1 1 0.568] Easter Egg
  (:`Pressed`
    (`|ExecutionSequence`
      (:`then_0`
        (goto _label_2 :!via `Close`))
      (:`then_1`
        (goto _label_3 :!via `Close`))
      (:`then_2`
        (goto _label :!via `Close`))
      (:`then_3`
        (`/Engine/EditorBlueprintResources/StandardMacros.Gate` true :!label _label_4
          (:`Exit`
            (goto _label_5 :!via `Open`)))))))

(event `Key|U`
  (params (Key :type "Key Structure"))
  ;[1 1 1 0.568] Easter Egg
  (:`Pressed`
    (`|ExecutionSequence`
      (:`then_0`
        (goto _label_2 :!via `Close`))
      (:`then_1`
        (goto _label_3 :!via `Close`))
      (:`then_2`
        (goto _label :!via `Close`))
      (:`then_3`
        (goto _label_4 :!via `Close`))
      (:`then_4`
        (`/Engine/EditorBlueprintResources/StandardMacros.Gate` true :!label _label_5
          (:`Exit`
            (bind _returnvalue (`|CreateWidget` "/Game/Blueprint/UI_UWU.UI_UWU_C" null self))
            (`UserWidget.AddToViewport` _returnvalue 0)))))))

(event `Key|Enter`
  (params (Key :type "Key Structure"))
  ;[1 1 1 0.568] Easter Egg
  (:`Pressed`
    (bind _result (`/Engine/EditorBlueprintResources/StandardMacros.IncrementInt` (`self.TimePressed`))
      (:`  `
        (if (>= _result 5)
          (goto _label_2 :!via `Open`))))))

(event `RemoveUI`
  (params (Target :type "Widget Object Reference"))
  ;[1 0.1754 0.5361] Remove UI
  (`Widget.RemoveFromParent` Target))

(fn `UserConstructionScript`)